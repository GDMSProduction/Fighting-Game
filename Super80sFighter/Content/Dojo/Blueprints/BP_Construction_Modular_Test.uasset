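; Test modular construction piece for the Dojo that turns into a floor, wall or ceiling mesh based on its rotation.
; The construction script runs Check, which compares mesh world roll and pitch against wall and ceiling thresholds in sequence, so later matches override earlier ones.
; Change swaps the mesh, copies its rotation to the actor and applies a yaw offset for walls.
; The Flip input is unused, and both negative-angle wall conditions can never be true.
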(event EventBeginPlay)

(event Collision|EventActorBeginOverlap
  (params (OtherActor :type Actor%20Object%20Reference)))

(event EventTick
  (params (DeltaSeconds :type Float%20%28single-precision%29)))

(fn ConstructionScript
  (CallFunction|Check))

(fn Check
  (bind _mesh (Variables|Default|GetMesh))
  (bind _threshold_wall (Variables|Default|GetThreshold_Wall))
  (bind _threshold_ceiling (Variables|Default|GetThreshold_Ceiling))
  (bind _returnvalue (Transformation|GetWorldRotation _mesh))
  (bind (_roll _pitch) (Math|Rotator|BreakRotator _returnvalue))
  (Utilities|FlowControl|Sequence
    (:then_0
      ;[1 1 1] Floor
      (if (and (>= _roll 0.0) (< _roll _threshold_wall))
        (CallFunction|Change "Floor" false)
        (elif (and (< _roll 0.0) (> _roll (* _threshold_wall -1.0)))
          (CallFunction|Change "Floor" true))))
    (:then_1
      (if (and (<= _pitch 0.0) (< _pitch _threshold_wall))
        (CallFunction|Change "Floor" false)
        (elif (and (< _pitch 0.0) (> _threshold_wall (* _threshold_ceiling -1.0)))
          (CallFunction|Change "Floor" true))))
    (:then_2
      ;[1 1 1] Comment
      (if (and (> _roll _threshold_wall) (< _roll _threshold_ceiling))
        (CallFunction|Change "Wall" true 180)
        (elif (and (> _roll (* _threshold_ceiling -1.0)) (< _roll (* _threshold_ceiling -1.0)))
          (CallFunction|Change "Wall" false))))
    (:then_3
      (if (and (> _pitch _threshold_wall) (< _pitch _threshold_ceiling))
        (CallFunction|Change "Wall" true -90)
        (elif (and (> _pitch (* _threshold_ceiling -1.0)) (< _pitch (* _threshold_ceiling -1.0)))
          (CallFunction|Change "Wall" false 90))))
    (:then_4
      ;[1 1 1] Ceiling Values
      (if (or (> _roll _threshold_ceiling) (< _roll (* _threshold_ceiling -1.0)))
        (CallFunction|Change "Ceiling" true)))
    (:then_5
      (if (or (> _pitch _threshold_ceiling) (< _pitch (* _threshold_ceiling -1.0)))
        (CallFunction|Change "Ceiling" true)))))

(fn Change
  (params (ChangeMesh :type String) (Flip :type Boolean) (AdjustRot :type Integer))
  (bind _mesh (Variables|Default|GetMesh))
  (if (Utilities|Enum|Equal(Enum) ChangeMesh "Wall")
    (Components|StaticMesh|SetStaticMesh _mesh "/Game/Dojo/Wall/Dojo_wall.Dojo_wall")
    (Transformation|SetActorRotation (Transformation|GetWorldRotation _mesh))
    (Rendering|Material|SetMaterial _mesh 0 0)
    (Transformation|SetRelativeRotation _mesh (Math|Rotator|MakeRotator 0.0 0.0 (Math|Conversions|ToFloat(Integer) AdjustRot)) false false)
    (elif (Utilities|Enum|Equal(Enum) ChangeMesh "Floor")
      (Components|StaticMesh|SetStaticMesh _mesh "/Game/Geometry/Meshes/TemplateFloor.TemplateFloor")
      (Transformation|SetActorRotation (Transformation|GetWorldRotation _mesh))
      (Rendering|Material|SetMaterial _mesh 0 0)
      (elif (Utilities|Enum|Equal(Enum) ChangeMesh "Ceiling")
        (Components|StaticMesh|SetStaticMesh _mesh "/Game/StarterContent/Architecture/Floor_400x400.Floor_400x400")
        (Transformation|SetActorRotation (Transformation|GetWorldRotation _mesh))
        (Rendering|Material|SetMaterial _mesh 0 0)))))